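; BP_WeaponTemplate_Pistol is a hitscan pistol weapon Blueprint that damages whatever its shot hits.
; ProcessFiring line-traces on the Visibility channel from FirePoint along its forward vector out to Range, ignoring the owner, and applies DamagePerHit to the hit actor.
; BeginPlay calls Fire automatically once after a short delay, and the trace draws timed debug lines.
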(event `self.ReceiveBeginPlay`
  (`KismetSystemLibrary.Delay` 3.0)
  (`self.Fire`))

(event `self.ProcessFiring`
  (bind _firepoint (`self.FirePoint`))
  (bind _returnvalue (`SceneComponent.K2_GetComponentLocation` _firepoint))
  (bind (_outhit _returnvalue_2) (`KismetSystemLibrary.LineTraceSingle` _returnvalue (+ _returnvalue (* (`SceneComponent.GetForwardVector` _firepoint) (`self.Range`))) "TraceTypeQuery1" false (`|MakeArray` (`self.GetOwner`)) "ForDuration"))
  (if _returnvalue_2
    (`GameplayStatics.ApplyDamage` (`.HitActor` (`GameplayStatics.BreakHitResult` _outhit)) (`self.DamagePerHit`))))

(fn `UserConstructionScript`)