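; Shotgun weapon Blueprint for the sandbox that overrides the fire event to shoot a spread of pellets.
; Each shot passes ammo and fire-readiness checks, then fires several line traces in random directions within a cone around the fire point and updates ammo.
; A HandleFireDelay timer gates the next shot, though its RoF division has a zero numerator.
; A failed ammo check triggers a reload and sound.
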(event `self.SandboxFire`
  (if (`self.CanFire`)
    (bind _returnvalue (`self.CheckAmmo`))
    (if _returnvalue
      (`|ExecutionSequence`
        (:`then_0`
          (`self.PlaySound` null)
          (for _ (range 7)
            (`self.LinetraceOneShot` (`KismetMathLibrary.RandomUnitVectorInConeInDegrees` (`SceneComponent.GetForwardVector` (`self.FirePoint`)) 20.0)))
          (`self.UpdateAmmo`))
        (:`then_1`
          (bind _returnvalue_2 (`KismetSystemLibrary.K2_SetTimer` null "HandleFireDelay" (/ 0.0 (`self.RoF`))))
          (set `self.TimerFireDelay` _returnvalue_2)
          (set `self.CanFire` false)))
      (else
        (`self.Reload`)
        (`self.PlaySound` null)))))

(fn `UserConstructionScript`)